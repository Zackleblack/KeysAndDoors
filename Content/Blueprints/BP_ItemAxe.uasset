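; Axe item Blueprint that the first-person character can hold, swing, drop or throw.
; Pickup attaches the mesh to the player's hand socket, while drop detaches it with physics, and use delegates to the player's SwingAxe.
; Secondary use runs the drop logic, launches the axe along camera forward and updates the inventory component.
; Throwing also binds to BP_Gate's hit event, sending BreakableMessage to hit actors implementing BPI_Breakable.
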(event Custom|CustomEvent
  (params (SelfActor :type Actor%20Object%20Reference) (OtherActor :type Actor%20Object%20Reference) (NormalImpulse :type Vector) (Hit :type Hit%20Result%20Structure%20%28by%20ref%29))
  (bind _hitactor (Collision|BreakHitResult Hit))
  (if (Utilities|DoesObjectImplementInterface _hitactor "/Game/Blueprints/BPI_Breakable.BPI_Breakable_C")
    (Class|BPIBreakable|Breakable(Message) _hitactor)))

(event EventBeginPlay
  (bind _asbp_first_person_character (Utilities|Casting|CastToBP_FirstPersonCharacter (Game|GetPlayerCharacter 0)))
  (bind _output_get (Variables|Default|SetPlayer%20REF _asbp_first_person_character))
  (Utilities|FlowControl|Delay 0.1)
  (bind _returnvalue (Actor|GetActorOfClass "/Game/Blueprints/BP_Gate.BP_Gate_C"))
  (Variables|Default|SetGATE%20REF _returnvalue))

(event Collision|EventActorBeginOverlap
  (params (OtherActor :type Actor%20Object%20Reference)))

(event EventTick
  (params (DeltaSeconds :type Float%20%28single-precision%29)))

(event EventSecondaryUse
  (bind _axe (Variables|Default|GetAxe))
  (Utilities|FlowControl|Sequence
    (:then_0
      (Development|PrintString "Dropping AXE")
      (Transformation|DetachFromComponent (Variables|Default|GetAxe) "KeepWorld" "KeepWorld" "KeepWorld" true)
      (Physics|SetSimulatePhysics (Variables|Default|GetAxe) true)
      (Collision|SetCollisionEnabled (Variables|Default|GetAxe) "QueryAndPhysics")
      (Variables|/Game/FirstPerson/Blueprints/BP_FirstPersonCharacter.BP_FirstPersonCharacter_C|SetbIsHoldingItem? (stale EventBeginPlay _output_get) false))
    (:then_1
      (bind _output_get (Variables|/Game/FirstPerson/Blueprints/BP_FirstPersonCharacter.BP_FirstPersonCharacter_C|SetbIsHoldingItem? (stale EventBeginPlay _output_get) false))
      (Development|PrintString (Utilities|String|ToString(Boolean) _output_get))
      (Variables|/Game/FirstPerson/Blueprints/BP_FirstPersonCharacter.BP_FirstPersonCharacter_C|SetHit%20Actor (stale EventBeginPlay _output_get) 0)
      (Development|PrintString "AXE HAS BEEN THROWN" true true "(R=1.000000,G=0.000000,B=0.105208,A=1.000000)")
      (Transformation|DetachFromComponent _axe "KeepWorld" "KeepWorld" "KeepWorld" true)
      (Physics|SetSimulatePhysics _axe true)
      (Collision|SetCollisionEnabled (Variables|Default|GetAxe) "QueryAndPhysics")
      (Physics|AddImpulse (Variables|Default|GetAxe) (* (Math|Vector|GetForwardVector (Camera|GetCameraRotation (Game|GetPlayerCameraManager 0))) 1.5e+03) "None" true)
      (Collision|BindEventtoOnActorHit (Variables|Default|GetGATE%20REF) (delegate Custom|CustomEvent)))
    (:then_2
      (Default|ActortoHitActorUpdateEvent (Variables|/Game/FirstPerson/Blueprints/BP_FirstPersonCharacter.BP_FirstPersonCharacter_C|GetBPC_InventorySystem (Variables|Default|GetPlayer%20REF))))))

(event EventDropItem
  (Development|PrintString "Dropping AXE")
  (Transformation|DetachFromComponent (Variables|Default|GetAxe) "KeepWorld" "KeepWorld" "KeepWorld" true)
  (Physics|SetSimulatePhysics (Variables|Default|GetAxe) true)
  (Collision|SetCollisionEnabled (Variables|Default|GetAxe) "QueryAndPhysics")
  (Variables|/Game/FirstPerson/Blueprints/BP_FirstPersonCharacter.BP_FirstPersonCharacter_C|SetbIsHoldingItem? (stale EventBeginPlay _output_get) false))

(event EventPickupItem
  (params (Hit%20Actor :type Actor%20Object%20Reference))
  (bind _axe (Variables|Default|GetAxe))
  (Collision|SetCollisionEnabled _axe "NoCollision")
  (bind _returnvalue (Transformation|AttachComponentToComponent _axe (Variables|/Game/FirstPerson/Blueprints/BP_FirstPersonCharacter.BP_FirstPersonCharacter_C|GetFirstPersonMesh (stale EventBeginPlay _output_get)) "Hand_r" "SnapToTarget" "SnapToTarget" "KeepWorld" true))
  (Variables|/Game/FirstPerson/Blueprints/BP_FirstPersonCharacter.BP_FirstPersonCharacter_C|SetbIsHoldingItem? (stale EventBeginPlay _output_get) _returnvalue))

(event EventUseItem
  (Default|SwingAxe (Variables|Default|GetPlayer%20REF)))

(fn ConstructionScript)