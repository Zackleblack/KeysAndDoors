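; BP_BombItem is a throwable bomb item for the inventory system, showing a "Pick Up Bomb" prompt when looked at.
; UseItem prints a debug message, detaches the cube, enables physics and collision, and launches it along player 0's camera forward with a mass-independent impulse.
; DropItem asks the inventory component to unequip through its server call.
; No detonation or damage logic is present.
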(event EventBeginPlay
  (|CallParentFunction) ; This node is disabled and will not be called.\nDrag off pins to build functionality.
)

(event Collision|EventActorBeginOverlap
  (params (OtherActor :type Actor%20Object%20Reference))
  (|CallParentFunction OtherActor) ; This node is disabled and will not be called.\nDrag off pins to build functionality.
)

(event EventTick
  (params (DeltaSeconds :type Float%20%28single-precision%29))
  (|CallParentFunction DeltaSeconds) ; This node is disabled and will not be called.\nDrag off pins to build functionality.
)

(event EventUseItem
  (Development|PrintString "BOMB HAS BEEN Thrown" true true "(R=1.000000,G=0.000000,B=0.105208,A=1.000000)")
  (Transformation|DetachFromComponent (Variables|Default|GetCube) "KeepWorld" "KeepWorld" "KeepWorld" true)
  (Physics|SetSimulatePhysics (Variables|Default|GetCube) true)
  (Collision|SetCollisionEnabled (Variables|Default|GetCube) "QueryAndPhysics")
  (Physics|AddImpulse (Variables|Default|GetCube) (* (Math|Vector|GetForwardVector (Camera|GetCameraRotation (Game|GetPlayerCameraManager 0))) 1e+03) "None" true))

(event EventDropItem
  (Default|SERVERUnequip (Variables|Default|GetBPC_InventorySystem)))

(fn ConstructionScript
  (|CallParentFunction))

(fn Lookingat
  (return "Pick Up Bomb"))