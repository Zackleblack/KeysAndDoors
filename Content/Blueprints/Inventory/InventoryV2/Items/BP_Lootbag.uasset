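; BP_Lootbag is a loot bag actor with an inventory component that removes itself once it is empty.
; On each inventory update it checks the component's quantity.
; At zero or below, it casts player controller 0 to BP_FirstPersonPlayerController, removes that HUD's Menu widget from its parent, then destroys itself.
; If the cast fails, the bag is not destroyed.
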(event OnInventoryUpdate(BPC_InventorySystem)
  (if (<= (Default|GetQuantity (Variables|Default|GetBPC_InventorySystem)) 0)
    (bind _asbp_first_person_player_controller (Utilities|Casting|CastToBP_FirstPersonPlayerController (Game|GetPlayerController 0)))
    (Widget|RemovefromParent (Variables|/Game/Blueprints/Inventory/InventoryV2/Widgets/WBP_PlayerHud.WBP_PlayerHud_C|GetMenu (Variables|/Game/FirstPerson/Blueprints/BP_FirstPersonPlayerController.BP_FirstPersonPlayerController_C|GetPlayer%20HUD _asbp_first_person_player_controller)))
    (Actor|DestroyActor)))

(event EventBeginPlay
  (|CallParentFunction) ; This node is disabled and will not be called.\nDrag off pins to build functionality.
)

(event Collision|EventActorBeginOverlap
  (params (OtherActor :type Actor%20Object%20Reference))
  (|CallParentFunction OtherActor) ; This node is disabled and will not be called.\nDrag off pins to build functionality.
)

(event EventTick
  (params (DeltaSeconds :type Float%20%28single-precision%29))
  (|CallParentFunction DeltaSeconds) ; This node is disabled and will not be called.\nDrag off pins to build functionality.
)

(fn ConstructionScript
  (|CallParentFunction))