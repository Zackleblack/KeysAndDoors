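; Inventory component that stores stackable item slots and handles player interaction, equipping, consuming and dropping items.
; DT_ItemDataTable drives stack limits and item classes for adding, slot transfers, hand-socket equipping and effect spawning, with multi-item drops placed in a lootbag.
; A per-tick camera sphere trace sets the look-at actor and prompt, which the interact input uses.
; Inventory updates trigger saving through the GameInstance's save object, reloaded on BeginPlay.
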(event Custom|Multitask%20update
  ;[0.15 0.15 0.15 0.5] Multi Task Update
  (Default|CallOnInventoryUpdate))

(event Custom|Server%20interact
  (params (Target :type Actor%20Object%20Reference))
  (bind _returnvalue (Components|GetOwner))
  (bind _returnvalue_2 (Actor|GetComponentbyClass Target "/Game/Blueprints/Inventory/InventoryV2/BPC_ItemData.BPC_ItemData_C"))
  (bind _asbp_first_person_character (Utilities|Casting|CastToBP_FirstPersonCharacter _returnvalue))
  (Utilities|IsValid _returnvalue_2
    (:Is%20Valid
      (Class|BPIInteractive|Interactwith(Message) _returnvalue_2 (.AsBP%20First%20Person%20Character (Utilities|Casting|CastToBP_FirstPersonCharacter (Components|GetOwner)))))
    (:Is%20Not%20Valid
      (Actor|SetOwner Target (Pawn|GetController _asbp_first_person_character))
      (CallFunction|OnLocalInteract Target _asbp_first_person_character))))

(event Custom|Unequip%20Item
  (Variables|Default|SetEquipped false))

(event Custom|Actor%20to%20Hit%20Actor%20Update_Event
  (Variables|Default|SetEquipped false))

(event Custom|Server%20Transfer
  (params (Source%20Index :type Integer) (Source%20Inventory :type BPC%20Inventory%20System%20Object%20Reference) (Destination%20Index :type Integer))
  ;[0.15 0.15 0.15 0.5] Transfering Slots
  (CallFunction|TransferSlots Source%20Index Source%20Inventory Destination%20Index))

(event Custom|On%20Local%20Interact
  (params (Target%20Actor :type Actor%20Object%20Reference) (Interactor :type Actor%20Object%20Reference))
  (Class|BPIInteractive|Interactwith(Message) Target%20Actor (.AsBP%20First%20Person%20Character (Utilities|Casting|CastToBP_FirstPersonCharacter Interactor))))

(event Custom|Server_DropItem
  (params (ItemID :type Name) (Quantity :type Integer))
  (if (> Quantity 1)
    (bind _returnvalue (Game|SpawnActorfromClass "/Game/Blueprints/Inventory/InventoryV2/Items/BP_Lootbag.BP_Lootbag_C" (Math|Transform|MakeTransform (CallFunction|GetDropLocation) "0, 0, 0" "1.000000,1.000000,1.000000") "AdjustIfPossibleButAlwaysSpawn" "MultiplyWithRoot" 0 0))
    (CallFunction|AddtoInventory (Variables|/Game/Blueprints/Inventory/InventoryV2/BP_Chest.BP_Chest_C|GetBPC_InventorySystem _returnvalue) ItemID Quantity)
    (else
      (Game|SpawnActorfromClass (.ItemClass (Utilities|Struct|BreakS_ItemStruct (CallFunction|GetItemData ItemID))) (Math|Transform|MakeTransform (CallFunction|GetDropLocation) "0, 0, 0" "1.000000,1.000000,1.000000") "AdjustIfPossibleButAlwaysSpawn" "MultiplyWithRoot" 0 0))))

(event Custom|Server_Remove
  (params (Index :type Integer) (Remove%20Whole%20Stack :type Boolean) (Is%20Consumed :type Boolean) (Equippable? :type Boolean))
  (CallFunction|RemovefromInventory Index Remove%20Whole%20Stack Is%20Consumed Equippable?))

(event Custom|Server%20Consumed
  (params (Item%20ID :type Name))
  (Game|SpawnActorfromClass (.ItemEffect (Utilities|Struct|BreakS_ItemStruct (CallFunction|GetItemData Item%20ID))) (Math|Transform|MakeTransform (CallFunction|GetDropLocation) "0, 0, 0" "1.000000,1.000000,1.000000") "Undefined" "MultiplyWithRoot" 0 0))

(event Custom|Server%20Equip
  (params (Item%20ID :type Name))
  (bind _data (CallFunction|GetItemData Item%20ID))
  (bind (_name _description _image _itemclass _stacksize _itemeffect _equipable_) (Utilities|Struct|BreakS_ItemStruct _data))
  (if (Variables|Default|GetEquipped)
    (Development|PrintString "You already have an Item Equipped")
    (elif _equipable_
      (bind _returnvalue (Game|SpawnActorfromClass _itemclass (Math|Transform|MakeTransform (Transformation|GetActorLocation (Game|GetPlayerCharacter 0)) "0, 0, 0" "0.500000,0.500000,0.500000") "AlwaysSpawn" "MultiplyWithRoot" 0 0))
      (bind _output_get (Variables|Default|SetEquipped%20Item _returnvalue))
      (bind _returnvalue_2 (Transformation|AttachComponentToComponent _output_get (Variables|/Script/Engine.Character|GetMesh (.AsBP%20First%20Person%20Character (Utilities|Casting|CastToBP_FirstPersonCharacter (Game|GetPlayerCharacter 0)))) "Hand_r" "SnapToTarget" "SnapToTarget" "KeepRelative" true))
      (Collision|SetActorEnableCollision _output_get _returnvalue_2)
      (Variables|Default|SetEquipped true)
      (Default|CallActortoHitActorUpdate))))

(event Custom|SERVER_Unequip
  (params (Equipped%20Actor :type Actor%20Object%20Reference))
  (Actor|DestroyActor Equipped%20Actor)
  (Variables|Default|SetEquipped%20Item 0)
  (Variables|Default|SetEquipped false)
  (CallFunction|AddtoInventory (.Name (Utilities|Struct|BreakS_ItemStruct (CallFunction|GetItemData (stale Custom|Server%20Equip Item%20ID)))) 1)
  (CallFunction|MultitaskUpdate))

(event Custom|Save%20Game
  (CallFunction|SaveInventory))

(event Input|EnhancedActionEvents|EnhancedInputActionIA_Interact
  (params (ActionValue :type Boolean) (ElapsedSeconds :type Float%20%28double-precision%29) (TriggeredSeconds :type Float%20%28double-precision%29) (InputAction :type Input%20Action%20Object%20Reference :default "/Game/Input/Actions/IA_Interact.IA_Interact"))
  (:Started
    (bind _look_at_actor (Variables|Default|GetLook%20At%20Actor)
      (:then
        (CallFunction|ServerInteract _look_at_actor))
      (:else))))

(event EventBeginPlay
  ;[0.15 0.15 0.15 0.5] Event Begin Play (Display Message)
  (CallFunction|LoadInventory)
  (Utilities|Array|Resize (Variables|Default|GetContent) (Variables|Default|GetInventory%20Size))
  (bind _returnvalue (UserInterface|CreateWidget "/Game/Blueprints/Inventory/InventoryV2/Widgets/WBP_DisplayMessage.WBP_DisplayMessage_C"))
  (bind _output_get (Variables|Default|SetDisplay%20Message _returnvalue))
  (UserInterface|Viewport|AddtoViewport _output_get 0)
  (Variables|Default|SetEquipped%20Item 0)
  (EventDispatchers|BindEventtoOnInventoryUpdate (delegate Custom|Save%20Game)))

(event EventTick
  (params (DeltaSeconds :type Float%20%28single-precision%29))
  ;[0.15 0.15 0.15 0.5] Trace Interaction
  (CallFunction|InteractionTrace))

(event Input|KeyboardEvents|1
  (params (Key :type Key%20Structure :default "None"))
  (:Pressed
    (CallFunction|DEBUG)))

(event Input|KeyboardEvents|2
  (params (Key :type Key%20Structure :default "None"))
  (:Pressed
    (Development|PrintString (Utilities|String|ToString(Boolean) (.Success (CallFunction|QueryInventory "TestItem" 2))))))

(event Input|KeyboardEvents|3
  (params (Key :type Key%20Structure :default "None"))
  (:Pressed
    (Development|PrintString (Utilities|GetDisplayName (Variables|Default|GetEquipped%20Item)))))

(fn AddtoInventory
  (params (Item%20ID :type Name) (Quantity :type Integer))
  (LocalVariables|SetLocal%20Quantity%20Remaining Quantity)
  (while (and (> (LocalVariables|GetLocal%20Quantity%20Remaining) 0) (not (LocalVariables|GetbLocal%20Has%20Failed)))
    (bind (_index _foundslot) (CallFunction|FindSlot Item%20ID))
    (if _foundslot
      (CallFunction|AddtoStack _index 1)
      (Math|Integer|DecrementInt (LocalVariables|GetLocal%20Quantity%20Remaining))
      (elif (.Has%20Empty%20Slot? (CallFunction|AnyEmptySlotsAvailable))
        (bind _success (CallFunction|CreateNewStack Item%20ID 1))
        (if _success
          (Math|Integer|DecrementInt (LocalVariables|GetLocal%20Quantity%20Remaining))
          (else
            (LocalVariables|SetbLocal%20Has%20Failed true)))
        (else
          (LocalVariables|SetbLocal%20Has%20Failed true)))))
  (Default|CallOnInventoryUpdate)
  (return (not (LocalVariables|GetbLocal%20Has%20Failed)) (LocalVariables|GetLocal%20Quantity%20Remaining)))

(fn RemovefromInventory
  (params (Index :type Integer) (Remove%20Whole%20Stack :type Boolean) (Is%20Consumed :type Boolean) (Equippable? :type Boolean))
  (bind _content (Variables|Default|GetContent))
  (bind _content_2 (Variables|Default|GetContent))
  (bind _content_3 (Variables|Default|GetContent))
  (bind _output (Utilities|Array|Get(acopy) _content Index))
  (bind _output_2 (Utilities|Array|Get(acopy) _content_3 Index))
  (bind _output_3 (Utilities|Array|Get(acopy) _content_2 Index))
  (LocalVariables|SetLocal%20Item (.itemid _output))
  (Variables|Default|SetLocal%20Quantity (.quanity _output))
  (Utilities|FlowControl|Sequence
    (:then_0
      (if (or Remove%20Whole%20Stack (== (Variables|Default|GetLocal%20Quantity) 1))
        (if Equippable?
          (if (Variables|Default|GetEquipped)
            (Development|PrintString "Actor is Already Equipped")
            (else
              (Utilities|Array|SetArrayElem (Variables|Default|GetContent) Index (Utilities|Struct|MakeS_SlotStruct "" 0))
              (CallFunction|ServerEquip (LocalVariables|GetLocal%20Item))
              (Development|PrintString "We are Equipping item")))
          (else
            (Utilities|Array|SetArrayElem (Variables|Default|GetContent) Index (Utilities|Struct|MakeS_SlotStruct "" 0))
            (if (not Is%20Consumed)
              (CallFunction|ServerDropItem (LocalVariables|GetLocal%20Item) (Variables|Default|GetLocal%20Quantity)))))
        (elif Equippable?
          (if (Variables|Default|GetEquipped)
            (Development|PrintString "Actor is Already Equipped")
            (else
              (Utilities|Struct|SetmembersinS_SlotStruct _output_2 (- (.Quanity (Utilities|Struct|BreakS_SlotStruct _output_2)) 1))
              (CallFunction|ServerEquip (LocalVariables|GetLocal%20Item))
              (Development|PrintString "We are Equipping item")))
          (else
            (Utilities|Struct|SetmembersinS_SlotStruct _output_3 (- (.Quanity (Utilities|Struct|BreakS_SlotStruct _output_3)) 1))
            (if (not Is%20Consumed)
              (CallFunction|ServerDropItem (LocalVariables|GetLocal%20Item) 1))))))
    (:then_1
      (CallFunction|MultitaskUpdate))))

(fn InteractionTrace
  (bind _returnvalue (Game|GetPlayerCameraManager 0))
  (bind _returnvalue_2 (Transformation|GetActorLocation _returnvalue))
  (bind (_outhit _returnvalue_3) (Collision|SphereTraceByChannel _returnvalue_2 (+ _returnvalue_2 (* (Transformation|GetActorForwardVector _returnvalue) 3e+02)) 5.0 "TraceTypeQuery4" false (Utilities|Array|MakeArray (Components|GetOwner)) "None"))
  (if _returnvalue_3
    (if (!= (.HitActor (Collision|BreakHitResult _outhit)) (Variables|Default|GetLook%20At%20Actor))
      (bind _output_get (Variables|Default|SetLook%20At%20Actor (.HitActor (Collision|BreakHitResult _outhit))))
      (bind _message (Class|BPIInteractive|Lookingat(Message) _output_get))
      (Default|ShowMessage (Variables|Default|GetDisplay%20Message) _message))
    (else
      (Variables|Default|SetLook%20At%20Actor 0)
      (Default|ShowMessage (Variables|Default|GetDisplay%20Message)))))

(fn Interact
  (params (Character :type Character%20Object%20Reference) (Actor :type Actor%20Object%20Reference)))

(fn FindSlot
  (params (ItemID :type Name))
  (for (_array_element _array_index) (Variables|Default|GetContent)
    (if (== (.ItemID (Utilities|Struct|BreakS_SlotStruct _array_element)) ItemID)
      (if (< (.Quanity (Utilities|Struct|BreakS_SlotStruct _array_element)) (CallFunction|GetMaxStackSize ItemID))
        (return _array_index true))))
  (return -1 false))

(fn GetMaxStackSize
  (params (ItemID :type Name))
  (bind _returnvalue (Utilities|GetDataTableRow "/Game/Blueprints/Inventory/InventoryV2/DT_ItemDataTable.DT_ItemDataTable" ItemID)
    (:then
      (return (.Stacksize (Utilities|Struct|BreakS_ItemStruct _returnvalue))))
    (:RowNotFound
      (return -1))))

(fn AddtoStack
  (params (Index :type Integer) (Quantity :type Integer))
  (bind _content (Variables|Default|GetContent))
  (bind _output (Utilities|Array|Get(acopy) _content Index))
  (Utilities|Array|SetArrayElem (Variables|Default|GetContent) Index (Utilities|Struct|MakeS_SlotStruct (.itemid _output) (+ (.quanity _output) Quantity))))

(fn AnyEmptySlotsAvailable
  (for (_array_element _array_index) (Variables|Default|GetContent)
    (if (== (.Quanity (Utilities|Struct|BreakS_SlotStruct _array_element)) 0)
      (return true _array_index)))
  (return false -1))

(fn CreateNewStack
  (params (Item%20ID :type Name) (Quantity :type Integer))
  (bind (_has_empty_slot_ _empty_index) (CallFunction|AnyEmptySlotsAvailable))
  (if _has_empty_slot_
    (Utilities|Array|SetArrayElem (Variables|Default|GetContent) _empty_index (Utilities|Struct|MakeS_SlotStruct Item%20ID Quantity))
    (return true)
    (else
      (return false))))

(fn DEBUG
  (for (_array_element _array_index) (Variables|Default|GetContent)
    (Development|PrintString (Utilities|String|Append (Utilities|String|ToString(Integer) _array_index) ":" (Utilities|String|ToString(Name) (.ItemID (Utilities|Struct|BreakS_SlotStruct _array_element))) " = " (Utilities|String|ToString(Integer) (.Quanity (Utilities|Struct|BreakS_SlotStruct _array_element)))))))

(fn TransferSlots
  (params (Source%20Index :type Integer) (Source%20Inventory :type BPC%20Inventory%20System%20Object%20Reference) (Destination%20Index :type Integer))
  (bind _content (Variables|Default|GetContent))
  (bind _output (Utilities|Array|Get(acopy) _content Destination%20Index))
  ;[0.15 0.15 0.15 0.5] Is the Content Slot <?
  (LocalVariables|SetLocal%20Slot%20Content (Utilities|Array|Get(acopy) (Variables|BPC_InventorySystem_C|GetContent Source%20Inventory) Source%20Index))
  (if (not (< Destination%20Index 0))
    ;[0.15 0.15 0.15 0.5] Is the Local Slot = to Destination Slot Struct
    (if (== (.ItemID (Utilities|Struct|BreakS_SlotStruct (LocalVariables|GetLocal%20Slot%20Content))) (.ItemID (Utilities|Struct|BreakS_SlotStruct (Utilities|Array|Get(acopy) (Variables|Default|GetContent) Destination%20Index))))
      ;[0.15 0.15 0.15 0.5] True =
      (Utilities|Array|SetArrayElem (Variables|BPC_InventorySystem_C|GetContent Source%20Inventory) Source%20Index (Utilities|Struct|MakeS_SlotStruct (select (> (Math|Integer|Clamp(Integer) (- (+ (.quanity (LocalVariables|GetLocal%20Slot%20Content)) (.quanity (Utilities|Array|Get(acopy) (Variables|Default|GetContent) Destination%20Index))) (CallFunction|GetMaxStackSize (.itemid (LocalVariables|GetLocal%20Slot%20Content)))) 0 (CallFunction|GetMaxStackSize (.itemid (LocalVariables|GetLocal%20Slot%20Content)))) 0) (.itemid (LocalVariables|GetLocal%20Slot%20Content)) "None") (Math|Integer|Clamp(Integer) (- (+ (.quanity (LocalVariables|GetLocal%20Slot%20Content)) (.quanity (Utilities|Array|Get(acopy) (Variables|Default|GetContent) Destination%20Index))) (CallFunction|GetMaxStackSize (.itemid (LocalVariables|GetLocal%20Slot%20Content)))) 0 (CallFunction|GetMaxStackSize (.itemid (LocalVariables|GetLocal%20Slot%20Content))))))
      (Utilities|Array|SetArrayElem (Variables|Default|GetContent) Destination%20Index (Utilities|Struct|MakeS_SlotStruct (.itemid (LocalVariables|GetLocal%20Slot%20Content)) (Math|Integer|Clamp(Integer) (+ (.quanity (LocalVariables|GetLocal%20Slot%20Content)) (.quanity _output)) 0 (CallFunction|GetMaxStackSize (.itemid _output)))))
      (CallFunction|MultitaskUpdate)
      (CallFunction|MultitaskUpdate Source%20Inventory)
      (else
        ;[0.15 0.15 0.15 0.5] Comment
        (Utilities|Array|SetArrayElem (Variables|BPC_InventorySystem_C|GetContent Source%20Inventory) Source%20Index (Utilities|Array|Get(acopy) (Variables|Default|GetContent) Destination%20Index))
        (Utilities|Array|SetArrayElem (Variables|Default|GetContent) Destination%20Index (LocalVariables|GetLocal%20Slot%20Content))
        (CallFunction|MultitaskUpdate)
        (CallFunction|MultitaskUpdate Source%20Inventory)))))

(fn GetItemData
  (params (Item%20ID :type Name))
  (bind _returnvalue (Utilities|GetDataTableRow "/Game/Blueprints/Inventory/InventoryV2/DT_ItemDataTable.DT_ItemDataTable" Item%20ID)
    (:then
      (return _returnvalue))))

(fn GetDropLocation
  (bind _returnvalue (Components|GetOwner))
  (bind _returnvalue_2 (Transformation|GetActorLocation _returnvalue))
  (bind _returnvalue_3 (Transformation|GetActorForwardVector _returnvalue))
  (bind _returnvalue_4 (Math|Random|RandomUnitVectorinConeinDegrees _returnvalue_3 3e+01))
  (bind _returnvalue_5 (* _returnvalue_4 1.5e+02))
  (bind _returnvalue_6 (+ _returnvalue_2 _returnvalue_5))
  (bind _outhit (Collision|LineTraceByChannel _returnvalue_6 (- _returnvalue_6 "0.000000,0.000000,1100.000000") "TraceTypeQuery1" false 0 "None"))
  (return (.Location (Collision|BreakHitResult _outhit))))

(fn ConsumeItem
  (params (Index :type Integer))
  (bind _content (Variables|Default|GetContent))
  (bind _output (Utilities|Array|Get(acopy) _content Index))
  (LocalVariables|SetLocal%20Item%20ID (.itemid _output))
  (LocalVariables|SetLocal%20Quanttity (.quanity _output))
  (Utilities|FlowControl|Sequence
    (:then_0
      (CallFunction|ServerRemove Index false true false)
      (CallFunction|ServerConsumed (LocalVariables|GetLocal%20Item%20ID)))
    (:then_1
      (CallFunction|MultitaskUpdate))))

(fn QueryInventory
  (params (Item%20ID :type Name) (Quantity :type Integer))
  (for _array_element (Variables|Default|GetContent)
    (if (== Item%20ID (.ItemID (Utilities|Struct|BreakS_SlotStruct _array_element)))
      (LocalVariables|SetRunning%20Total (+ (.Quanity (Utilities|Struct|BreakS_SlotStruct _array_element)) (LocalVariables|GetRunning%20Total)))))
  (return (>= (LocalVariables|GetRunning%20Total) Quantity) (LocalVariables|GetRunning%20Total)))

(fn GetQuantity
  (for _array_element (Variables|Default|GetContent)
    (LocalVariables|SetLocal%20Sum (+ (LocalVariables|GetLocal%20Sum) (.quanity _array_element))))
  (return (LocalVariables|GetLocal%20Sum)))

(fn SaveInventory
  (bind _asbp_game_instance (Utilities|Casting|CastToBP_GameInstance (Game|GetGameInstance)))
  (Variables|/Game/Blueprints/BP_SaveData.BP_SaveData_C|SetInventory%20Content (Variables|/Game/Blueprints/BP_GameInstance.BP_GameInstance_C|GetMy%20Data%20Save%20Ref _asbp_game_instance) (Variables|Default|GetContent))
  (SaveGame|SaveGametoSlot (Variables|/Game/Blueprints/BP_GameInstance.BP_GameInstance_C|GetMy%20Data%20Save%20Ref _asbp_game_instance) "MyData"))

(fn LoadInventory
  (bind _asbp_game_instance (Utilities|Casting|CastToBP_GameInstance (Game|GetGameInstance)))
  (Variables|Default|SetContent (Variables|/Game/Blueprints/BP_SaveData.BP_SaveData_C|GetInventory%20Content (Variables|/Game/Blueprints/BP_GameInstance.BP_GameInstance_C|GetMy%20Data%20Save%20Ref _asbp_game_instance))))