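; Test item actor for the V2 inventory that supplies a "Pick up" prompt naming the item.
; Its BPCItemData component holds an ItemID data table row handle, which is looked up to fill the prompt with the row's Name.
; LookAt and Looking At contain identical prompt logic, while the event graph and construction script do nothing and no pickup logic is present.
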(event EventBeginPlay)

(event Collision|EventActorBeginOverlap
  (params (OtherActor :type Actor%20Object%20Reference)))

(event EventTick
  (params (DeltaSeconds :type Float%20%28single-precision%29)))

(fn ConstructionScript)

(fn Lookat
  (bind _bpc_itemdata (Variables|Default|GetBPC_ItemData))
  (bind _itemid (Variables|/Game/Blueprints/Inventory/InventoryV2/BPC_ItemData.BPC_ItemData_C|GetItemID _bpc_itemdata))
  (bind _returnvalue (Utilities|GetDataTableRow (.datatable _itemid) (.rowname _itemid))
    (:then
      (return (Utilities|Text|FormatText "Pick up {Item}" (.Name (Utilities|Struct|BreakS_ItemStruct _returnvalue)))))))

(fn Lookingat
  (bind _bpc_itemdata (Variables|Default|GetBPC_ItemData))
  (bind _itemid (Variables|/Game/Blueprints/Inventory/InventoryV2/BPC_ItemData.BPC_ItemData_C|GetItemID _bpc_itemdata))
  (bind _returnvalue (Utilities|GetDataTableRow (.datatable _itemid) (.rowname _itemid))
    (:then
      (return (Utilities|Text|FormatText "Pick up {Item}" (.Name (Utilities|Struct|BreakS_ItemStruct _returnvalue)))))))