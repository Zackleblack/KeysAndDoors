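; BP_Chest is an interactable inventory chest that swings its lid open for the first-person character and shows its contents.
; BeginPlay creates a WBP_ChestM widget bound to Inventory and picks a random index of 0 or 1.
; Interact plays a timeline lerping the lid's world rotation, then adds the widget and prints the indexed item.
; Close reverses that timeline, with ChestOpened preventing the widget from reappearing.
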(event Custom|Close
  ;[0.15 0.15 0.15 0.5] Comment
  (Variables|Default|SetbChest%20Opened? false)
  (bind _chest_open_alpha (Timeline|Open%20Chest Reverse)
    (:Update
      (Transformation|SetWorldRotation (Variables|Default|GetTop%20Chest) (Math|Rotator|Lerp(Rotator) "0.000000,90.000000,0.000000" "0.000000,50.000000,0.000000" _chest_open_alpha) false false))
    (:Finished
      (if (Variables|Default|GetbChest%20Opened?)
        (UserInterface|Viewport|AddtoViewport (Variables|Default|GetCurrent%20Chest%20Widget%20REF) 0)
        (Development|PrintText (Utilities|Text|FormatText "First Item in the barrel is {name} 
Description: {Description}" (.NameofItem (Utilities|Struct|BreakS_Item (Utilities|Array|Get(acopy) (Variables|Default|GetInventory) (stale Custom|Chest%20Set _output_get)))) (.Description (Utilities|Struct|BreakS_Item (Utilities|Array|Get(acopy) (Variables|Default|GetInventory) (stale Custom|Chest%20Set _output_get))))) true true "(R=1.000000,G=0.501057,B=0.113828,A=1.000000)" 2e+01)
        (Utilities|FlowControl|DoOnce false) ; enters at Reset
      ))))

(event Custom|Chest%20Set
  (Utilities|FlowControl|DoOnce false
    (:Completed
      (bind _returnvalue (UserInterface|CreateWidget "/Game/Blueprints/Inventory/WBP_ChestM.WBP_ChestM_C" 0 (Variables|Default|GetInventory)))
      (Variables|Default|SetCurrent%20Chest%20Widget%20REF _returnvalue)
      (bind _output_get (Variables|Default|SetChest%20Index (Math|Random|RandomIntegerinRange 0 1))))))

(event EventInteract
  (params (Character :type Character%20Object%20Reference))
  ;[0.15 0.15 0.15 0.5] Comment
  (Utilities|Casting|CastToBP_FirstPersonCharacter Character)
  (Development|PrintString "Opening Chest")
  (Utilities|FlowControl|DoOnce false :!label _label
    (:Completed
      (Variables|Default|SetbChest%20Opened? true)
      (bind _chest_open_alpha (Timeline|Open%20Chest Play)
        (:Update
          (Transformation|SetWorldRotation (Variables|Default|GetTop%20Chest) (Math|Rotator|Lerp(Rotator) "0.000000,90.000000,0.000000" "0.000000,50.000000,0.000000" _chest_open_alpha) false false))
        (:Finished
          (if (Variables|Default|GetbChest%20Opened?)
            (UserInterface|Viewport|AddtoViewport (Variables|Default|GetCurrent%20Chest%20Widget%20REF) 0)
            (Development|PrintText (Utilities|Text|FormatText "First Item in the barrel is {name} 
Description: {Description}" (.NameofItem (Utilities|Struct|BreakS_Item (Utilities|Array|Get(acopy) (Variables|Default|GetInventory) (stale Custom|Chest%20Set _output_get)))) (.Description (Utilities|Struct|BreakS_Item (Utilities|Array|Get(acopy) (Variables|Default|GetInventory) (stale Custom|Chest%20Set _output_get))))) true true "(R=1.000000,G=0.501057,B=0.113828,A=1.000000)" 2e+01)
            (goto _label Reset)))))))

(event Collision|EventActorBeginOverlap
  (params (OtherActor :type Actor%20Object%20Reference)))

(event EventTick
  (params (DeltaSeconds :type Float%20%28single-precision%29))
  ;[0.15 0.15 0.15 0.5] Comment
)

(event EventBeginPlay
  ;[0.15 0.15 0.15 0.5] Comment
  (CallFunction|ChestSet))

(fn ConstructionScript)