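; BP_ExplodableRock is a rock that is removed from the world when its Explode event is called.
; Explode hands off to EXPLOSION, which turns off the Rock component's collision and destroys it, with debug prints along the way.
; EXPLOSION sets Hidden In Game to false before destruction and spawns no effects or debris.
; Nodes for a random mesh swap and a RockCluster reference sit unconnected.
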(event Custom|EXPLOSION
  (bind _rock (Variables|Default|GetRock))
  (Development|PrintString "ROCKS WERE HIT" true true "(R=1.000000,G=0.018550,B=0.000000,A=1.000000)" 5.0)
  (Development|SetHiddeninGame _rock false false)
  (Collision|SetCollisionEnabled _rock "NoCollision")
  (Components|DestroyComponent (Variables|Default|GetRock)))

(event EventBeginPlay)

(event EventExplode
  (Development|PrintString "Hello")
  (CallFunction|EXPLOSION))

(fn ConstructionScript)