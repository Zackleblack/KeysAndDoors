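; Throwable, placeable bomb item that the first-person player carries and detonates.
; BPI_Item events attach it to the hand socket or detach it with physics, either dropped, thrown along camera forward, or placed.
; Throwing and placing update the character's inventory component and start a short fuse.
; Detonation sphere-traces for BPI_Explode actors, sends them ExplodeMessage, plays Niagara and sound effects, then destroys the bomb.
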(event Custom|Interact_1_1
  (params (Character :type Character%20Object%20Reference)))

(event Custom|Explosion%20Timer%20Start
  (bind _bomb (Variables|Default|GetBomb))
  (bind _returnvalue (Transformation|GetWorldLocation _bomb))
  ;[0.15 0.15 0.15 0.5] Timer Start (Bomb Starts Ticking)
  (bind (_outhits _returnvalue_2) (Collision|MultiSphereTraceByChannel _returnvalue _returnvalue 2.5e+02 "TraceTypeQuery3" false 0 "None"))
  (for _array_element _outhits
    (if _returnvalue_2
      (Development|PrintString (Utilities|GetDisplayName (.HitActor (Collision|BreakHitResult _array_element))))
      (if (Utilities|DoesObjectImplementInterface (.HitActor (Collision|BreakHitResult _array_element)) "/Game/Blueprints/BPI_Explode.BPI_Explode_C")
        (Development|PrintString "BOMB HIT SOMETHING" true true "(R=1.000000,G=0.019433,B=0.000000,A=1.000000)" 5.0)
        (Class|BPIExplode|Explode(Message) (.HitActor (Collision|BreakHitResult _array_element))))))
  (Niagara|SpawnSystematLocation "/Game/Niagra/NS_Explosion.NS_Explosion" (Transformation|GetWorldLocation (Variables|Default|GetBomb)))
  (Audio|PlaySoundatLocation "/Game/Audio/Bombs/ExplosionSound.ExplosionSound" (Transformation|GetWorldLocation (Variables|Default|GetBomb)) "0, 0, 0" 1.0 1.0 0.0 "/Game/Audio/Bombs/Attenuation_Sphere.Attenuation_Sphere" 0 0 0)
  (Variables|/Game/FirstPerson/Blueprints/BP_FirstPersonCharacter.BP_FirstPersonCharacter_C|SetHit%20Actor (Variables|Default|GetFirst%20Person%20Character) 0)
  (Utilities|FlowControl|Delay 0.1)
  (Actor|DestroyActor))

(event EventBeginPlay
  ;[0.15 0.15 0.15 0.5] Save Player Reference
  (bind _asbp_first_person_character (Utilities|Casting|CastToBP_FirstPersonCharacter (Game|GetPlayerCharacter 0)))
  (Variables|Default|SetFirst%20Person%20Character _asbp_first_person_character))

(event EventDropItem
  ;[0.15 0.15 0.15 0.5] Drop Item (BPI_Item)
  (Development|PrintString "Dropping Bomb")
  (Transformation|DetachFromComponent (Variables|Default|GetBomb) "KeepWorld" "KeepWorld" "KeepWorld" true)
  (Physics|SetSimulatePhysics (Variables|Default|GetBomb) true)
  (Collision|SetCollisionEnabled (Variables|Default|GetBomb) "QueryAndPhysics")
  (Variables|/Game/FirstPerson/Blueprints/BP_FirstPersonCharacter.BP_FirstPersonCharacter_C|SetbIsHoldingItem? (Variables|Default|GetFirst%20Person%20Character) false))

(event EventPickupItem
  (params (Hit%20Actor :type Actor%20Object%20Reference))
  (bind _bomb (Variables|Default|GetBomb))
  ;[0.15 0.15 0.15 0.5] Pick Up Bomb (BPI_Item)
  (if (not (Variables|/Game/FirstPerson/Blueprints/BP_FirstPersonCharacter.BP_FirstPersonCharacter_C|GetbIsHoldingItem? (Variables|Default|GetFirst%20Person%20Character)))
    (Collision|SetCollisionEnabled _bomb "NoCollision")
    (bind _returnvalue (Transformation|AttachComponentToComponent _bomb (Variables|/Game/FirstPerson/Blueprints/BP_FirstPersonCharacter.BP_FirstPersonCharacter_C|GetFirstPersonMesh (Variables|Default|GetFirst%20Person%20Character)) "Hand_r" "SnapToTarget" "SnapToTarget" "KeepWorld" true))
    (Variables|/Game/FirstPerson/Blueprints/BP_FirstPersonCharacter.BP_FirstPersonCharacter_C|SetbIsHoldingItem? (Variables|Default|GetFirst%20Person%20Character) _returnvalue)))

(event EventUseItem
  (bind _first_person_character (Variables|Default|GetFirst%20Person%20Character))
  ;[0.15 0.15 0.15 0.5] Use Item (BPI_Item)
  (Development|PrintString "BOMB HAS BEEN Thrown" true true "(R=1.000000,G=0.000000,B=0.105208,A=1.000000)")
  (Transformation|DetachFromComponent (Variables|Default|GetBomb) "KeepWorld" "KeepWorld" "KeepWorld" true)
  (Physics|SetSimulatePhysics (Variables|Default|GetBomb) true)
  (Collision|SetCollisionEnabled (Variables|Default|GetBomb) "QueryAndPhysics")
  (Variables|/Game/FirstPerson/Blueprints/BP_FirstPersonCharacter.BP_FirstPersonCharacter_C|SetbIsHoldingItem? _first_person_character false)
  (Default|ActortoHitActorUpdateEvent (Variables|/Game/FirstPerson/Blueprints/BP_FirstPersonCharacter.BP_FirstPersonCharacter_C|GetBPC_InventorySystem _first_person_character))
  (Physics|AddImpulse (Variables|Default|GetBomb) (* (Math|Vector|GetForwardVector (Camera|GetCameraRotation (Game|GetPlayerCameraManager 0))) 1e+03) "None" true)
  (Utilities|FlowControl|Delay 1.0)
  (CallFunction|ExplosionTimerStart))

(event EventSecondaryUse
  ;[0.15 0.15 0.15 0.5] Drop Bomb (BPI_Item)
  (Default|ActortoHitActorUpdateEvent (Variables|/Game/FirstPerson/Blueprints/BP_FirstPersonCharacter.BP_FirstPersonCharacter_C|GetBPC_InventorySystem (Variables|Default|GetFirst%20Person%20Character)))
  (Development|PrintString "BOMB HAS BEEN PLACED" true true "(R=1.000000,G=0.000000,B=0.105208,A=1.000000)")
  (Transformation|DetachFromComponent (Variables|Default|GetBomb) "KeepWorld" "KeepWorld" "KeepWorld" true)
  (Physics|SetSimulatePhysics (Variables|Default|GetBomb) true)
  (Collision|SetCollisionEnabled (Variables|Default|GetBomb) "QueryAndPhysics")
  (Variables|/Game/FirstPerson/Blueprints/BP_FirstPersonCharacter.BP_FirstPersonCharacter_C|SetbIsHoldingItem? (Variables|Default|GetFirst%20Person%20Character) false)
  (Variables|/Game/FirstPerson/Blueprints/BP_FirstPersonCharacter.BP_FirstPersonCharacter_C|SetHit%20Actor (Variables|Default|GetFirst%20Person%20Character) 0)
  (Utilities|FlowControl|Delay 1.0)
  (CallFunction|ExplosionTimerStart))

(fn ConstructionScript)

(fn Interact
  (params (Character :type Character%20Object%20Reference) (Actor :type Actor%20Object%20Reference))
  (return))