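; BP_StumpAxe is a one-time interactable axe pickup that grants the axe to the first-person player.
; Interact plays a timeline that raises the axe, then a second timeline that pulls it toward the player and hides it after a short delay.
; When that finishes, it calls GetAxe on the cached player reference, then destroys the axe component and hides the Niagara aura.
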(event Custom|Get%20Axe
  (Default|GetAxe (Variables|Default|GetPlayer%20REF))
  (Utilities|FlowControl|Delay 0.2)
  (Components|DestroyComponent (Variables|Default|GetAxe))
  (Rendering|SetVisibility (Variables|Default|GetNS_MushroomAura_02) false false))

(event EventBeginPlay
  (bind _asbp_first_person_character (Utilities|Casting|CastToBP_FirstPersonCharacter (Game|GetPlayerCharacter 0)))
  (Variables|Default|SetPlayer%20REF _asbp_first_person_character))

(event Collision|EventActorBeginOverlap
  (params (OtherActor :type Actor%20Object%20Reference)))

(event EventTick
  (params (DeltaSeconds :type Float%20%28single-precision%29)))

(event EventInteract
  (params (Character :type Character%20Object%20Reference))
  (bind _axe (Variables|Default|GetAxe))
  (bind _returnvalue (Transformation|GetWorldLocation _axe))
  (Utilities|FlowControl|DoOnce false
    (:Completed
      (bind _lift_up (Timeline|Timeline Play)
        (:Update
          (Transformation|SetWorldLocation _axe (Math|Vector|Lerp(Vector) _returnvalue (+ _returnvalue "0.000000,0.000000,2.000000") _lift_up) false false))
        (:Finished
          (bind _spin (Timeline|Spin PlayFromStart)
            (:Update
              (Transformation|SetWorldLocation (Variables|Default|GetAxe) (Math|Vector|Lerp(Vector) (Transformation|GetWorldLocation (Variables|Default|GetAxe)) (Transformation|GetActorLocation (Variables|Default|GetPlayer%20REF)) _spin) false false)
              (Utilities|FlowControl|Delay 0.5)
              (Development|SetHiddeninGame (Variables|Default|GetAxe) true false))
            (:Finished
              (CallFunction|GetAxe))))))))

(fn ConstructionScript)