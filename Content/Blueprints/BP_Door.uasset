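; BP_Door is a key-locked door that the first-person player can interact with while inside its overlap box.
; With the key, a FlipFlop alternates opening and closing sounds and a yaw timeline, disabling collision during the swing.
; Without it, a rate-limited thought widget appears.
; A one-time Breakable event leaves an axe visible in the door, stops the melee montage, shows a failure thought and destroys the axe item.
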(event OnComponentBeginOverlap(Box)
  (params (OverlappedComponent :type Primitive%20Component%20Object%20Reference) (OtherActor :type Actor%20Object%20Reference) (OtherComp :type Primitive%20Component%20Object%20Reference) (OtherBodyIndex :type Integer) (bFromSweep :type Boolean) (SweepResult :type Hit%20Result%20Structure%20%28by%20ref%29))
  (Utilities|Casting|CastToBP_FirstPersonCharacter OtherActor)
  (Variables|Default|SetbAmINearDoor? true)
  (Development|PrintString "Near Door = True"))

(event OnComponentEndOverlap(Box)
  (params (OverlappedComponent :type Primitive%20Component%20Object%20Reference) (OtherActor :type Actor%20Object%20Reference) (OtherComp :type Primitive%20Component%20Object%20Reference) (OtherBodyIndex :type Integer))
  (Utilities|Casting|CastToBP_FirstPersonCharacter OtherActor)
  (Variables|Default|SetbAmINearDoor? false)
  (Development|PrintString "Near Door = False"))

(event Custom|Key%20Get!
  (Variables|Default|SetbHasKey? true))

(event Custom|Door%20Stuck
  (Development|SetHiddeninGame (Variables|Default|GetAxe) false false)
  (Animation|StopAnimMontage (Variables|Default|GetCharacter%20Reference) "/Game/Animation/BergsAnim/Melee_Attack_AM.Melee_Attack_AM")
  (bind _returnvalue (UserInterface|CreateWidget "/Game/Widgets/WBP_Thoughts.WBP_Thoughts_C"))
  (Rendering|Components|TextRender|SetText (Variables|/Game/Widgets/WBP_Thoughts.WBP_Thoughts_C|GetTextBox _returnvalue) "You: Welp, that didn't work...")
  (UserInterface|Viewport|AddtoViewport _returnvalue 0)
  (Utilities|FlowControl|Sequence
    (:then_0
      (Utilities|FlowControl|Delay 5.0)
      (Widget|RemovefromParent _returnvalue))
    (:then_1
      (Variables|/Game/FirstPerson/Blueprints/BP_FirstPersonCharacter.BP_FirstPersonCharacter_C|SetHit%20Actor (Variables|Default|GetCharacter%20Reference) 0)
      (Actor|DestroyActor (Variables|Default|GetAxe%20REF))
      (Variables|/Game/FirstPerson/Blueprints/BP_FirstPersonCharacter.BP_FirstPersonCharacter_C|SetbIsHoldingItem? (Variables|Default|GetCharacter%20Reference) false))))

(event EventBeginPlay
  (bind _asbp_first_person_character (Utilities|Casting|CastToBP_FirstPersonCharacter (Game|GetPlayerCharacter 0)))
  (Variables|Default|SetCharacter%20Reference _asbp_first_person_character)
  (Utilities|FlowControl|Delay 0.2)
  (bind _returnvalue (Actor|GetActorOfClass "/Game/Blueprints/BP_ItemAxe.BP_ItemAxe_C"))
  (Variables|Default|SetAxe%20REF _returnvalue))

(event Collision|EventActorBeginOverlap
  (params (OtherActor :type Actor%20Object%20Reference)))

(event EventTick
  (params (DeltaSeconds :type Float%20%28single-precision%29)))

(event EventInteract
  (params (Character :type Character%20Object%20Reference))
  (bind _door (Variables|Default|GetDoor))
  (bind _relativerotation (Variables|/Script/Engine.SceneComponent|GetRelativeRotation _door))
  (if (Variables|Default|GetbAmINearDoor?)
    (if (Variables|Default|GetbHasKey?)
      (Utilities|FlowControl|DoOnce false :!label _label
        (:Completed
          (Utilities|FlowControl|FlipFlop
            (:A
              (Audio|PlaySound2D "/Game/Audio/DoorSFX/DoorOpen_Cue.DoorOpen_Cue" 1.0 1.0 0.0 0 0)
              (bind _opening (Timeline|DoorOpening PlayFromStart)
                (:Update
                  (Utilities|FlowControl|Sequence
                    (:then_0
                      (Transformation|SetRelativeRotation _door (Math|Rotator|MakeRotator (.roll _relativerotation) (.pitch _relativerotation) (Math|Float|Lerp -9e+01 -1.8e+02 _opening)) false false))
                    (:then_1
                      (Utilities|FlowControl|DoOnce false :!label _label_2
                        (:Completed
                          (Collision|SetCollisionEnabled _door "NoCollision"))))))
                (:Finished
                  (Utilities|FlowControl|Sequence
                    (:then_0
                      (goto _label_2 Reset))
                    (:then_1
                      (Collision|SetCollisionEnabled (Variables|Default|GetDoor) "QueryAndPhysics")
                      (goto _label Reset))))))
            (:B
              (Audio|PlaySound2D "/Game/Audio/DoorSFX/DoorClose_Cue.DoorClose_Cue" 1.0 1.0 0.0 0 0)
              (Timeline|DoorOpening ReverseFromEnd)))))
      (else
        (Utilities|FlowControl|DoOnce false :!label _label_3
          (:Completed
            (bind _returnvalue (UserInterface|CreateWidget "/Game/Widgets/WBP_Thoughts.WBP_Thoughts_C"))
            (UserInterface|Viewport|AddtoViewport _returnvalue 0)
            (Utilities|FlowControl|Delay 5.0)
            (goto _label_3 Reset)))))))

(event EventBreakable
  (Utilities|FlowControl|DoOnce false
    (:Completed
      (CallFunction|DoorStuck))))

(fn ConstructionScript)