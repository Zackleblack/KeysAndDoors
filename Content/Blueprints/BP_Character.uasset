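; BP_Character is an animated character that plays a looping animation and moves itself vertically through a timeline.
; BeginPlay starts the AnimationToPlay clip on the mesh, then calls the Movement event, which plays the timeline.
; Each timeline update offsets the actor from its current location by up to a small Z step scaled by the track value, so movement accumulates without sweeping for collision.
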(event Custom|Movement
  (bind _self self)
  (bind _returnvalue (Transformation|GetActorTransform _self))
  (bind _newtrack_0 (Timeline|Timeline Play)
    (:Update
      (Transformation|SetActorLocation (Math|Vector|Lerp(Vector) (.location _returnvalue) (+ (.location _returnvalue) "0.000000,0.000000,5.000000") _newtrack_0) false false))))

(event EventBeginPlay
  (Components|Animation|PlayAnimation (Variables|Character|GetMesh) (Variables|Default|GetAnimation%20to%20play) true)
  (CallFunction|Movement))

(event Collision|EventActorBeginOverlap
  (params (OtherActor :type Actor%20Object%20Reference)))

(event EventTick
  (params (DeltaSeconds :type Float%20%28single-precision%29)))

(fn ConstructionScript)