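; BP_SecurityCamera is a security camera that uses AI Perception to spot targets and raise an alarm.
; Perception updates not tagged "AI" print the sensed class and feed HandleSight.
; On detection, it swaps the camera material, plays a sound at the player's location and sends every BP_DumDum to check the stimulus location.
; Losing the target switches to another material, with debug prints throughout.
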(event OnTargetPerceptionUpdated(AIPerception)
  (params (Actor :type Actor%20Object%20Reference) (Stimulus :type AI%20Stimulus%20Structure))
  (bind (_age _expirationage _strength _stimuluslocation _receiverlocation _tag _bsuccessfullysensed) (Utilities|Struct|BreakAIStimulus Stimulus))
  (if (not (== _tag "AI"))
    (bind _returnvalue (Class|AIPerceptionSystem|GetSenseClassforStimulus Stimulus))
    (Development|PrintText (Utilities|Text|FormatText "Sensed: {ACtor} with {NAME}" (Utilities|GetClassDisplayName _returnvalue) Actor))
    (switch string (Utilities|GetClassDisplayName _returnvalue)
      (:AISense_Sight
        (CallFunction|HandleSight Actor _bsuccessfullysensed _stimuluslocation)))))

(event OnTargetPerceptionForgotten(AIPerception)
  (params (Actor :type Actor%20Object%20Reference))
  (Development|PrintString "I forgor"))

(event OnTargetPerceptionInfoUpdated(AIPerception)
  (params (UpdateInfo :type Actor%20Perception%20Update%20Info%20Structure%20%28by%20ref%29)))

(event EventBeginPlay)

(event Collision|EventActorBeginOverlap
  (params (OtherActor :type Actor%20Object%20Reference)))

(event EventTick
  (params (DeltaSeconds :type Float%20%28single-precision%29)))

(fn ConstructionScript)

(fn HandleSight
  (params (Target :type Actor%20Object%20Reference) (Successfully%20Sensed :type Boolean) (Handle%20Sight :type Vector))
  (bind _camera (Variables|Default|GetCamera))
  (if Successfully%20Sensed
    (Development|PrintText "Acquired Target")
    (Rendering|Material|SetMaterial _camera 0 "/Engine/EngineMaterials/EditorBrushMaterial.EditorBrushMaterial")
    (Audio|PlaySoundatLocation "/Game/Blueprints/AI/tindeck_1.tindeck_1" (Transformation|GetActorLocation (Game|GetPlayerCharacter 0)) "0, 0, 0" 1.0 1.0 0.0 "/Game/Audio/Bombs/Attenuation_Sphere.Attenuation_Sphere" 0 0 0)
    (bind _outactors (Actor|GetAllActorsOfClass "/Game/Blueprints/AI/BP_DumDum.BP_DumDum_C"))
    (for _array_element _outactors
      (Default|CheckOutSecurityAlarm _array_element Handle%20Sight))
    (else
      (Development|PrintText "Lost Target")
      (Rendering|Material|SetMaterial _camera 0 "/Engine/MapTemplates/Materials/BasicAsset03.BasicAsset03"))))