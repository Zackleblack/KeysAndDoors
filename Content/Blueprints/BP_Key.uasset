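; BP_Key is a one-time key pickup that grants the key to a referenced Door when interacted with.
; Interact runs through a DoOnce, calls KeyGet on the door, hides the key mesh and plays a sound.
; It then shows a WBP_ItemGet widget with the key's name, icon and hint.
; BeginPlay starts a Spin timeline, but the rotation and DestroyActor nodes are disconnected, so the actor only hides.
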(event EventBeginPlay
  (bind _newtrack_0 (Timeline|Spin Play)))

(event EventTick
  (params (DeltaSeconds :type Float%20%28single-precision%29)))

(event EventInteract
  (params (Character :type Character%20Object%20Reference))
  (Utilities|FlowControl|DoOnce false
    (:Completed
      (Default|KeyGet! (Variables|Default|GetDoor%20))
      (Development|SetHiddeninGame (Variables|Default|GetKey) true false)
      (Audio|PlaySound2D "/Engine/EditorSounds/Notifications/CompileSuccess.CompileSuccess" 1.0 1.0 0.0 0 0)
      (bind _returnvalue (UserInterface|CreateWidget "/Game/Widgets/WBP_ItemGet.WBP_ItemGet_C"))
      (Rendering|Components|TextRender|SetText (Variables|/Game/Widgets/WBP_ItemGet.WBP_ItemGet_C|Gettooltip _returnvalue) "Looks like this can open a door!")
      (Rendering|Components|TextRender|SetText (Variables|/Game/Widgets/WBP_ItemGet.WBP_ItemGet_C|GetITEMNAME _returnvalue) "Door Key!")
      (Appearance|SetBrushfromTexture (Variables|/Game/Widgets/WBP_ItemGet.WBP_ItemGet_C|GetITEMBOX _returnvalue) "/Game/Door_Key.Door_Key" false)
      (UserInterface|Viewport|AddtoViewport _returnvalue 0))))

(fn ConstructionScript)